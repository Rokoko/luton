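; Bartender character Blueprint that initializes its animation Blueprint when play begins.
; It passes its ActorName to the bartender anim instance on the skeletal mesh.
; It also switches the anim instance's EnablePhysics off, then back on after a short delay, so physics starts slightly after spawn.
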(event `self.ReceiveBeginPlay`
  (`|ExecutionSequence`
    (:`then_0`
      (bind _asbartender_anim_bp (cast `/Game/Characters/Bartender/bartender_animBP` (`SkeletalMeshComponent.GetAnimInstance` (`self.SkeletalMesh`))))
      (set `/Game/Characters/Bartender/bartender_animBP.ActorName` (`self.ActorName`) _asbartender_anim_bp))
    (:`then_1`
      (bind _asbartender_anim_bp_2 (cast `/Game/Characters/Bartender/bartender_animBP` (`SkeletalMeshComponent.GetAnimInstance` (`self.SkeletalMesh`))))
      (set `/Game/Characters/Bartender/bartender_animBP.Enable Physics` false _asbartender_anim_bp_2)
      (`KismetSystemLibrary.Delay` 0.2)
      (set `/Game/Characters/Bartender/bartender_animBP.Enable Physics` true _asbartender_anim_bp_2))))

(fn `UserConstructionScript`)