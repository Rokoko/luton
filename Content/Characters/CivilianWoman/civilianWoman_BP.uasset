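; Civilian woman character Blueprint that configures its animation Blueprint, civilianWoman_animBP, when play begins.
; It passes its ActorName to the anim instance on its skeletal mesh.
; It then switches the anim instance's EnablePhysics flag off and turns it back on after a short delay.
; Tick, overlap and construction script contain no logic.
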(event `self.ReceiveBeginPlay`
  (`|ExecutionSequence`
    (:`then_0`
      (bind _ascivilian_woman_anim_bp (cast `/Game/Characters/CivilianWoman/civilianWoman_animBP` (`SkeletalMeshComponent.GetAnimInstance` (`self.SkeletalMesh`))))
      (set `/Game/Characters/CivilianWoman/civilianWoman_animBP.ActorName` (`self.ActorName`) _ascivilian_woman_anim_bp))
    (:`then_1`
      (bind _ascivilian_woman_anim_bp_2 (cast `/Game/Characters/CivilianWoman/civilianWoman_animBP` (`SkeletalMeshComponent.GetAnimInstance` (`self.SkeletalMesh`))))
      (set `/Game/Characters/CivilianWoman/civilianWoman_animBP.Enable Physics` false _ascivilian_woman_anim_bp_2)
      (`KismetSystemLibrary.Delay` 0.2)
      (set `/Game/Characters/CivilianWoman/civilianWoman_animBP.Enable Physics` true _ascivilian_woman_anim_bp_2))))

(fn `UserConstructionScript`)