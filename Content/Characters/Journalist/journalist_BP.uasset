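; Journalist character Blueprint that initializes its animation Blueprint, journalist_AnimBP, when play begins.
; It turns the anim instance's EnablePhysics flag off, then back on after a short delay, apparently to hold off animation physics during spawn.
; It also copies its ActorName into the anim instance, and has no other active logic.
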(event `self.ReceiveBeginPlay`
  (`|ExecutionSequence`
    (:`then_0`
      (bind _asjournalist_anim_bp (cast `/Game/Characters/Journalist/journalist_AnimBP` (`SkeletalMeshComponent.GetAnimInstance` (`self.SkeletalMesh`))))
      (set `/Game/Characters/Journalist/journalist_AnimBP.Enable Physics` false _asjournalist_anim_bp)
      (`KismetSystemLibrary.Delay` 0.2)
      (set `/Game/Characters/Journalist/journalist_AnimBP.Enable Physics` true _asjournalist_anim_bp))
    (:`then_1`
      (bind _asjournalist_anim_bp_2 (cast `/Game/Characters/Journalist/journalist_AnimBP` (`SkeletalMeshComponent.GetAnimInstance` (`self.SkeletalMesh`))))
      (set `/Game/Characters/Journalist/journalist_AnimBP.ActorName` (`self.ActorName`) _asjournalist_anim_bp_2))))

(fn `UserConstructionScript`)