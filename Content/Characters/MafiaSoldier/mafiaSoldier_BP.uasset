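; Mafia soldier character Blueprint that initializes its animation Blueprint when play begins.
; It turns the anim instance's EnablePhysics flag off, then back on after a short delay.
; It also passes its ActorName to the anim instance.
; Overlap, tick and the construction script are empty.
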(event `self.ReceiveBeginPlay`
  (`|ExecutionSequence`
    (:`then_0`
      (bind _asmafia_soldier_anim_bp (cast `/Game/Characters/MafiaSoldier/mafiaSoldier_AnimBP` (`SkeletalMeshComponent.GetAnimInstance` (`self.SkeletalMesh`))))
      (set `/Game/Characters/MafiaSoldier/mafiaSoldier_AnimBP.Enable Physics` false _asmafia_soldier_anim_bp)
      (`KismetSystemLibrary.Delay` 0.2)
      (set `/Game/Characters/MafiaSoldier/mafiaSoldier_AnimBP.Enable Physics` true _asmafia_soldier_anim_bp))
    (:`then_1`
      (bind _asmafia_soldier_anim_bp_2 (cast `/Game/Characters/MafiaSoldier/mafiaSoldier_AnimBP` (`SkeletalMeshComponent.GetAnimInstance` (`self.SkeletalMesh`))))
      (set `/Game/Characters/MafiaSoldier/mafiaSoldier_AnimBP.ActorName` (`self.ActorName`) _asmafia_soldier_anim_bp_2))))

(fn `UserConstructionScript`)