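; Waitress character Blueprint that initializes its animation Blueprint, waitress_animBP, when play begins.
; It switches the anim instance's EnablePhysics flag off, then back on after a short delay.
; It also passes its ActorName to the anim instance; all other logic is empty.
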(event `self.ReceiveBeginPlay`
  (`|ExecutionSequence`
    (:`then_0`
      (bind _aswaitress_anim_bp (cast `/Game/Characters/Waitress/waitress_animBP` (`SkeletalMeshComponent.GetAnimInstance` (`self.SkeletalMesh`))))
      (set `/Game/Characters/Waitress/waitress_animBP.Enable Physics` false _aswaitress_anim_bp)
      (`KismetSystemLibrary.Delay` 0.2)
      (set `/Game/Characters/Waitress/waitress_animBP.Enable Physics` true _aswaitress_anim_bp))
    (:`then_1`
      (bind _aswaitress_anim_bp_2 (cast `/Game/Characters/Waitress/waitress_animBP` (`SkeletalMeshComponent.GetAnimInstance` (`self.SkeletalMesh`))))
      (set `/Game/Characters/Waitress/waitress_animBP.ActorName` (`self.ActorName`) _aswaitress_anim_bp_2))))

(fn `UserConstructionScript`)